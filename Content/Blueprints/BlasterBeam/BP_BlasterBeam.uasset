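; BP_BlasterBeam is a blaster beam actor that ends the game when it hits its target pawn.
; BeginPlay binds the mesh's component hit event to HandleOnHit, which spawns the NS_BeamBurst Niagara effect at the impact point, oriented along the surface normal.
; If the hit actor matches TargetPawn it quits the game outright, otherwise the beam destroys itself.
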(event `self.ReceiveBeginPlay`
  (add `PrimitiveComponent.OnComponentHit` (`self.Mesh`) (delegate `OnComponentHit_Event`)))

(event `OnComponentHit_Event`
  (params (HitComponent :type "PrimitiveComponent Object Reference") (OtherActor :type "Actor Object Reference") (OtherComp :type "PrimitiveComponent Object Reference") (NormalImpulse :type "Vector Structure") (Hit :type "HitResult Structure (by ref)"))
  (`self.HandleOnHit` OtherActor Hit))

(fn `HandleOnHit`
  (params (OtherActor :type "Object Object Reference") (Hit :type "HitResult Structure (by ref)"))
  (bind (_bblockinghit _binitialoverlap _time _distance _location _impactpoint _normal) (`GameplayStatics.BreakHitResult` Hit))
  (`NiagaraFunctionLibrary.SpawnSystemAtLocation` "/Game/Assets/FX/NS_BeamBurst.NS_BeamBurst" _impactpoint (`KismetMathLibrary.MakeRotFromX` _normal))
  ; Eğer oyuncuya çarptıysan oyunu sonlandır. Eğer oyuncuya çarpmadıysan ışın aktörünü yok et.
  (if (== (`local.OtherActor`) (`self.TargetPawn`))
    (`KismetSystemLibrary.QuitGame` null "Quit")
    (else
      (`self.K2_DestroyActor`))))

(fn `UserConstructionScript`)